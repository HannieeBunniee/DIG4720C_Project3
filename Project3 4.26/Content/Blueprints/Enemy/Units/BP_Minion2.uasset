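; BP_Minion2 is a tank-bodied lane minion unit with a health bar widget.
; Damage reduces its health, updates the bar and destroys the actor at zero.
; On begin play a looping timer replays a timeline that rocks the tank body with a random roll.
; After a short delay it copies waypoints for its team and lane from GM_Main; this graph does not move it along them.
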(event `self.ReceiveAnyDamage`
  (params (Damage :type "Float (single-precision)") (DamageType :type "DamageType Object Reference") (InstigatedBy :type "Controller Object Reference") (DamageCauser :type "Actor Object Reference"))
  ;[1 1 1] Take Damage
  (bind _output_get (set `self.CurrentHealth` (- (`self.CurrentHealth`) Damage)))
  (`/Game/Widget/UI_EnemyHealthBar.Update HP Bar` (`self.Enemy HP Ref`) (`self.CurrentHealth`) (`self.MaxHealth`))
  (if (<= _output_get 0.0)
    (`self.K2_DestroyActor`)))

(event `self.ReceiveBeginPlay`
  (`|ExecutionSequence`
    (:`then_0`
      ;[1 1 1] HP
      (bind _returnvalue (`|CreateWidget` "/Game/Widget/UI_EnemyHealthBar.UI_EnemyHealthBar_C"))
      (bind _output_get (set `self.Enemy HP Ref` _returnvalue))
      (`WidgetComponent.SetWidget` (`self.HealthWidget`) _output_get)
      (`self.PlayAnimation`)
      (`KismetSystemLibrary.K2_SetTimerDelegate` (delegate `PlayAnimation`) 1.0 true))
    (:`then_1`
      (`KismetSystemLibrary.Delay` 0.2)
      (bind _asgm_main (cast `/Game/GameFiles/GM_Main` (`GameplayStatics.GetGameMode`)))
      (bind _output_get_2 (set `self.GameMode` _asgm_main))
      (bind _waypoint (`/Game/GameFiles/GM_Main.GetWaypointsForMinion` _output_get_2 (`self.Team`) (`self.Lane`)))
      (for (_array_element _array_index) _waypoint
        (`KismetArrayLibrary.Array_Set` (`self.Waypoints`) _array_index _array_element true)))))

(event `PlayAnimation`
  ;[1 1 1] Animation for the Tank.
  (bind (_direction _alpha) (`Timeline|T_TankBodyAnimation` :!via `PlayFromStart`)
    (:`Update`
      (`SceneComponent.K2_SetRelativeRotation` (`self.Tank Body`) (`KismetMathLibrary.RLerp` (struct) (`KismetMathLibrary.MakeRotator` (`KismetMathLibrary.RandomFloatInRange` 2.0 5.0)) _alpha) false false))))

(fn `UserConstructionScript`)