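; BP_Monster is an enemy that chases the player, deals contact damage and gives health back when killed.
; Entering AttackRadius triggers AIMoveTo toward the player.
; Touching Collision starts a looping timer, never cleared here, that repeatedly damages the stored player reference.
; AnyDamage lowers health, crediting the player and destroying the monster at zero, while BeginPlay assigns an enemy health bar widget.
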(event `self.ReceiveAnyDamage`
  (params (Damage :type "Float (single-precision)") (DamageType :type "DamageType Object Reference") (InstigatedBy :type "Controller Object Reference") (DamageCauser :type "Actor Object Reference"))
  ;[1 1 1] Take Damage
  (set `self.CurrentHealth` (- (`self.CurrentHealth`) Damage))
  (if (<= (`self.CurrentHealth`) 0.0)
    ;[1 1 1] regend hp to player
    (bind _returnvalue (`GameplayStatics.GetActorOfClass` "/Game/Blueprints/Character/BP_PlayerCharacter.BP_PlayerCharacter_C"))
    (set `/Game/Blueprints/Character/BP_PlayerCharacter.CurrentHealth` (+ (`/Game/Blueprints/Character/BP_PlayerCharacter.CurrentHealth` _returnvalue) (`self.HealthGiveBack`)) _returnvalue)
    (`self.K2_DestroyActor`)))

(event `self.AttackRadius.OnComponentBeginOverlap`
  (params (OverlappedComponent :type "PrimitiveComponent Object Reference") (OtherActor :type "Actor Object Reference") (OtherComp :type "PrimitiveComponent Object Reference") (OtherBodyIndex :type Integer) (bFromSweep :type Boolean) (SweepResult :type "HitResult Structure (by ref)"))
  ;[1 1 1] Overlaps
  (bind _asbp_player_character (cast `/Game/Blueprints/Character/BP_PlayerCharacter` OtherActor))
  (`|AIMoveTo` self (0.0 0.0 0.0) _asbp_player_character))

(event `self.Collision.OnComponentBeginOverlap`
  (params (OverlappedComponent :type "PrimitiveComponent Object Reference") (OtherActor :type "Actor Object Reference") (OtherComp :type "PrimitiveComponent Object Reference") (OtherBodyIndex :type Integer) (bFromSweep :type Boolean) (SweepResult :type "HitResult Structure (by ref)"))
  ;[1 1 1] Damage To player if collide
  (bind _asbp_player_character (cast `/Game/Blueprints/Character/BP_PlayerCharacter` OtherActor))
  (set `self.PlayerRef` _asbp_player_character)
  (`KismetSystemLibrary.K2_SetTimerDelegate` (delegate `Damage Player`) 1.0 true))

(event `Damage Player`
  (bind _playerref (`self.PlayerRef`))
  ;[1 1 1] Damage To player if collide
  (`/Engine/EditorBlueprintResources/StandardMacros.IsValid` _playerref
    (:`Is Valid`
      (`GameplayStatics.ApplyDamage` _playerref (`self.DamageToPlayer`)))))

(event `self.ReceiveBeginPlay`
  ;[1 1 1] HP
  (bind _returnvalue (`|CreateWidget` "/Game/Widget/UI_EnemyHealthBar.UI_EnemyHealthBar_C"))
  (bind _output_get (set `self.HealthWidRef` _returnvalue))
  (`WidgetComponent.SetWidget` (`self.HealthWidget1`) _output_get))

(fn `UserConstructionScript`)