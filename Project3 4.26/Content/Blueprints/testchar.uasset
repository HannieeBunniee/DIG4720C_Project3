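; Automated turret that tracks and shoots actors carrying its attack team tag, and is destroyed when damage depletes its health.
; AttackRange overlaps maintain the ActorsInRange list, activating with a sound on entry and deactivating when no valid first target remains.
; While active, a timeline's update turns Head toward the first target and uses a Delay to throttle twin BP_TurretProjectile spawns at the left and right muzzle points.
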(event `self.ReceiveBeginPlay`
  (`|ExecutionSequence`
    (:`then_1`
      (`KismetArrayLibrary.Array_Clear` (`self.Actors in Range`)))))

(event `self.ReceiveAnyDamage`
  (params (Damage :type "Float (single-precision)") (DamageType :type "DamageType Object Reference") (InstigatedBy :type "Controller Object Reference") (DamageCauser :type "Actor Object Reference"))
  (bind _output_get (set `self.CurrentHealth` (- (`self.CurrentHealth`) Damage)))
  (if (<= _output_get 0.0)
    (`self.K2_DestroyActor`)
    (else
      (`KismetSystemLibrary.PrintString` "Turret Damaged"))))

(event `Activate`
  ;[1 1 1] Activate/Deactivate shooting
  (set `self.Activated` true)
  (`GameplayStatics.SpawnSoundAtLocation` null (`self.K2_GetActorLocation`) (struct) 1.0 1.0 0.0 null null) ; play sound when player come near
  (`Timeline|Timeline_0` :!label _label
    (:`Update`
      (`|ExecutionSequence`
        (:`then_0`
          (`self.LookAtPlayer`))
        (:`then_1`
          (`KismetSystemLibrary.Delay` (`self.FireRate`))
          (if (`self.Activated`)
            (`self.ShootAtPlayer`)))))))

(event `Deactivate`
  ;[1 1 1] Activate/Deactivate shooting
  (set `self.Activated` false)
  (goto _label :!via `Stop`))

(event `self.AttackRange.OnComponentBeginOverlap`
  (params (OverlappedComponent :type "PrimitiveComponent Object Reference") (OtherActor :type "Actor Object Reference") (OtherComp :type "PrimitiveComponent Object Reference") (OtherBodyIndex :type Integer) (bFromSweep :type Boolean) (SweepResult :type "HitResult Structure (by ref)"))
  ;[1 1 1] Event overlapse and exit
  (if (`self.ActorHasTag` OtherActor (`self.AttackTeam`))
    (`KismetArrayLibrary.Array_Add` (`self.Actors in Range`) OtherActor)
    (`self.Activate`)))

(event `self.AttackRange.OnComponentEndOverlap`
  (params (OverlappedComponent :type "PrimitiveComponent Object Reference") (OtherActor :type "Actor Object Reference") (OtherComp :type "PrimitiveComponent Object Reference") (OtherBodyIndex :type Integer))
  (bind _actors_in_range (`self.Actors in Range`))
  ;[1 1 1] Event overlapse and exit
  (if (`self.ActorHasTag` OtherActor (`self.AttackTeam`))
    (`KismetArrayLibrary.Array_RemoveItem` _actors_in_range OtherActor)
    (`/Engine/EditorBlueprintResources/StandardMacros.IsValid` (`|GetArrayItem` _actors_in_range)
      (:`Is Not Valid`
        (`self.Deactivate`)))))

(fn `LookAtPlayer`
  (bind _output (`|GetArrayItem` (`self.Actors in Range`)))
  (`/Engine/EditorBlueprintResources/StandardMacros.IsValid` _output
    (:`Is Valid`
      (`SceneComponent.K2_SetWorldRotation` (`self.Head`) (`KismetMathLibrary.FindLookAtRotation` (`SceneComponent.K2_GetComponentLocation` (`self.Head`)) (`self.K2_GetActorLocation` _output)) false false))))

(fn `ShootAtPlayer`
  (bind (_returnvalue_location _returnvalue_rotation _returnvalue_scale) (`KismetMathLibrary.BreakTransform` (`SceneComponent.K2_GetComponentToWorld` (`self.SpawnPointLeft`))))
  (bind (_returnvalue_location_2 _returnvalue_rotation_2 _returnvalue_scale_2) (`KismetMathLibrary.BreakTransform` (`SceneComponent.K2_GetComponentToWorld` (`self.SpawnPointRight`))))
  (`|SpawnActorFromClass` "/Game/Blueprints/Projectiles/BP_TurretProjectile.BP_TurretProjectile_C" (`KismetMathLibrary.MakeTransform` _returnvalue_location_2 _returnvalue_rotation_2 _returnvalue_scale_2) "AlwaysSpawn" "OverrideRootScale" null null)
  (`|SpawnActorFromClass` "/Game/Blueprints/Projectiles/BP_TurretProjectile.BP_TurretProjectile_C" (`KismetMathLibrary.MakeTransform` _returnvalue_location _returnvalue_rotation _returnvalue_scale) "AlwaysSpawn" "OverrideRootScale" null null))

(fn `UserConstructionScript`)