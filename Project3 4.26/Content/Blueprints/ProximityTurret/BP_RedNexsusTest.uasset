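; Red Nexus test actor that acts as a destructible objective, ending the game in a win when its health runs out.
; On begin play it disables collision on its Nexux component and creates a turret health widget, which is not added to the viewport here.
; Damage lowers health and updates that widget's bar.
; At zero it shows the win screen and mouse cursor, pauses the game, plays victory audio and destroys itself.
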(event `self.ReceiveBeginPlay`
  (`PrimitiveComponent.SetCollisionEnabled` (`self.nexux`) "NoCollision")
  (bind _returnvalue (`|CreateWidget` "/Game/Widget/UI_TurretHeath.UI_TurretHeath_C"))
  (set `self.WidgetRef` _returnvalue))

(event `self.ReceiveAnyDamage`
  (params (Damage :type "Float (single-precision)") (DamageType :type "DamageType Object Reference") (InstigatedBy :type "Controller Object Reference") (DamageCauser :type "Actor Object Reference"))
  (set `self.Current Health` (- (`self.Current Health`) Damage))
  (`/Game/Widget/UI_TurretHeath.update HP bar` (`self.WidgetRef`) (`self.Current Health`) (`self.MaxHealth`))
  (if (<= (`self.Current Health`) 0.0)
    ;[1 1 1] WON
    (bind _returnvalue (`|CreateWidget` "/Game/Widget/UI_Won.UI_Won_C"))
    (`UserWidget.AddToViewport` _returnvalue 0)
    (set `PlayerController.bShowMouseCursor` true (`GameplayStatics.GetPlayerController` 0))
    (`GameplayStatics.SetGamePaused` true)
    (`GameplayStatics.PlaySound2D` "/Game/Sounds/SFX/Victory.Victory" 1.0 1.0 0.0 null null)
    (`self.K2_DestroyActor`)))

(fn `UserConstructionScript`)