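; BP_MinionShot is a team-affiliated projectile that colors its bullet mesh red or blue by team and destroys itself after a short lifetime.
; On hit, it damages enemy minions, spawns a Niagara explosion matching the victim's team, then destroys itself.
; Same-team minion hits are ignored, while any non-minion actor takes damage without a team check or explosion and also destroys the shot.
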(event `self.ReceiveBeginPlay`
  (bind _sm_bullet (`self.SM_Bullet`))
  (if (== (`self.TeamAffiliation`) 0)
    (`PrimitiveComponent.SetMaterial` _sm_bullet 0 "/Game/Materials/M_SolidColor_Red.M_SolidColor_Red")
    (else
      (`PrimitiveComponent.SetMaterial` _sm_bullet 0 "/Game/Materials/M_SolidColor_Blue.M_SolidColor_Blue")))
  (`KismetSystemLibrary.Delay` 1.5)
  (`self.K2_DestroyActor`))

(event `self.ReceiveHit`
  (params (MyComp :type "PrimitiveComponent Object Reference") (Other :type "Actor Object Reference") (OtherComp :type "PrimitiveComponent Object Reference") (bSelfMoved :type Boolean) (HitLocation :type "Vector Structure") (HitNormal :type "Vector Structure") (NormalImpulse :type "Vector Structure") (Hit :type "HitResult Structure (by ref)"))
  (bind _asbp_minion (cast `/Game/Blueprints/Enemy/Units/BP_Minion` Other)
    (:`then`
      (bind _team (`/Game/Blueprints/Enemy/Units/BP_Minion.Team` _asbp_minion))
      (if (!= _team (`self.TeamAffiliation`))
        (`GameplayStatics.ApplyDamage` Other 20.0)
        (if (== _team 0)
          (`NiagaraFunctionLibrary.SpawnSystemAtLocation` "/Game/Particles/PS_Explosion_System.PS_Explosion_System" HitLocation)
          (else
            (`NiagaraFunctionLibrary.SpawnSystemAtLocation` "/Game/Particles/PS_Explosion_SystemBLUE.PS_Explosion_SystemBLUE" HitLocation)))
        (`self.K2_DestroyActor`)))
    (:`CastFailed`
      (`GameplayStatics.ApplyDamage` Other 20.0)
      (`self.K2_DestroyActor`))))

(fn `UserConstructionScript`)