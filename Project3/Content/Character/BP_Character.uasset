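; BP_Character is a player-driven tank character with hull movement and independently aimed turret and barrel, driven by axis input.
; MoveRight turns the hull by changing control rotation yaw, while MoveForward adds movement along that rotation's forward vector, yaw-offset by its own axis value.
; LookRight yaws the TankTurret locally, and LookUp elevates the TankBarrel through local roll rather than pitch, each with its own speed variable.
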(event `InputAxis|MoveForward`
  (params (AxisValue :type "Float (single-precision)"))
  ;[1 1 1] Movement
  (`self.AddMovementInput` (`KismetMathLibrary.GetForwardVector` (`KismetMathLibrary.MakeRotator` (.roll (`Controller.GetControlRotation` (`self.GetController`))) (.pitch (`Controller.GetControlRotation` (`self.GetController`))) (+ (.yaw (`Controller.GetControlRotation` (`self.GetController`))) (* (stale `InputAxis|MoveRight` AxisValue) (`self.TurnSpeed`))))) AxisValue))

(event `InputAxis|MoveRight`
  (params (AxisValue :type "Float (single-precision)"))
  (bind _returnvalue (`self.GetController`))
  ;[1 1 1] Movement
  (`Controller.SetControlRotation` _returnvalue (`KismetMathLibrary.MakeRotator` (.roll (`Controller.GetControlRotation` _returnvalue)) (.pitch (`Controller.GetControlRotation` _returnvalue)) (+ (.yaw (`Controller.GetControlRotation` _returnvalue)) (* AxisValue (`self.TurnSpeed`))))))

(event `InputAxis|LookRight`
  (params (AxisValue :type "Float (single-precision)"))
  (`SceneComponent.K2_AddLocalRotation` (`self.TankTurret`) (`KismetMathLibrary.MakeRotator` 0.0 0.0 (* AxisValue (`self.LookSpeedX`))) false false))

(event `InputAxis|LookUp`
  (params (AxisValue :type "Float (single-precision)"))
  (`SceneComponent.K2_AddLocalRotation` (`self.TankBarrel`) (`KismetMathLibrary.MakeRotator` (* AxisValue (`self.LookSpeedY`))) false false))

(fn `UserConstructionScript`)