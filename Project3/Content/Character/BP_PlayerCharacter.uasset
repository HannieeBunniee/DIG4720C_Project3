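; Player-controlled tank character that drives, aims, fires projectiles and takes damage, showing a game-over screen and pausing at zero health.
; Move axes steer the control rotation and drive the tank forward, while look axes independently rotate the turret and pitch the barrel.
; Left click spawns a projectile at SpawnPoint.
; While any axis is active, Tick draws a predicted-path debug trace from there, using a hard-coded speed meant to match the projectile's.
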(event `Key|LeftMouseButton`
  (params (Key :type "Key Structure"))
  ;[1 1 1] Shoot
  (:`Pressed`
    (`|SpawnActorFromClass` "/Game/Blueprints/Projectors/BP_PlayerProjectile.BP_PlayerProjectile_C" (`KismetMathLibrary.MakeTransform` (`SceneComponent.K2_GetComponentLocation` (`self.SpawnPoint`)) (`SceneComponent.K2_GetComponentRotation` (`self.SpawnPoint`))) "Undefined" "OverrideRootScale" null null)))

(event `self.ReceiveAnyDamage`
  (params (Damage :type "Float (single-precision)") (DamageType :type "DamageType Object Reference") (InstigatedBy :type "Controller Object Reference") (DamageCauser :type "Actor Object Reference"))
  ;[1 1 1] Taking Damage
  (set `self.CurrentHealth` (- (`self.CurrentHealth`) Damage))
  (if (<= (`self.CurrentHealth`) 0.0)
    ;;[1 1 1] Lose Screen
    (bind _returnvalue (`|CreateWidget` "/Game/Widget/UI_GameOver.UI_GameOver_C"))
    (`UserWidget.AddToViewport` _returnvalue 0)
    (set `PlayerController.bShowMouseCursor` true (`GameplayStatics.GetPlayerController` 0))
    (`GameplayStatics.SetGamePaused` true)))

(event `InputAxis|MoveForward`
  (params (AxisValue :type "Float (single-precision)"))
  ;[1 1 1] Movement
  (`self.AddMovementInput` (`KismetMathLibrary.GetForwardVector` (`KismetMathLibrary.MakeRotator` (.roll (`Controller.GetControlRotation` (`self.GetController`))) (.pitch (`Controller.GetControlRotation` (`self.GetController`))) (+ (.yaw (`Controller.GetControlRotation` (`self.GetController`))) (* (stale `InputAxis|MoveRight` AxisValue) (`self.TurnSpeed`))))) AxisValue))

(event `self.ReceiveBeginPlay`
  ;[1 1 1] Player HP
  (if (not (`self.IsMainMenu?`))
    (bind _returnvalue (`|CreateWidget` "/Game/Widget/UI_PlayerHUD.UI_PlayerHUD_C"))
    (`UserWidget.AddToViewport` _returnvalue 0)))

(event `self.ReceiveTick`
  (params (DeltaSeconds :type "Float (single-precision)"))
  ;[1 1 1] Have dots when player move/looks
  (if (or (!= (`self.GetInputAxisValue`) 0.0) (!= (`self.GetInputAxisValue`) 0.0) (!= (`self.GetInputAxisValue`) 0.0) (!= (`self.GetInputAxisValue`) 0.0))
    (`self.Aiming Dots`)))

(event `InputAxis|MoveRight`
  (params (AxisValue :type "Float (single-precision)"))
  (bind _returnvalue (`self.GetController`))
  ;[1 1 1] Movement
  (`Controller.SetControlRotation` _returnvalue (`KismetMathLibrary.MakeRotator` (.roll (`Controller.GetControlRotation` _returnvalue)) (.pitch (`Controller.GetControlRotation` _returnvalue)) (+ (.yaw (`Controller.GetControlRotation` _returnvalue)) (* AxisValue (`self.TurnSpeed`))))))

(event `InputAxis|LookRight`
  (params (AxisValue :type "Float (single-precision)"))
  ;[1 1 1] Looking
  (`SceneComponent.K2_AddLocalRotation` (`self.TankTurret`) (`KismetMathLibrary.MakeRotator` 0.0 0.0 (* AxisValue (`self.LookSpeedX`))) false false))

(event `InputAxis|LookUp`
  (params (AxisValue :type "Float (single-precision)"))
  ;[1 1 1] Looking
  (`SceneComponent.K2_AddLocalRotation` (`self.TankBarrel`) (`KismetMathLibrary.MakeRotator` (* AxisValue (`self.LookSpeedY`))) false false))

(fn `Aiming Dots`
  (`GameplayStatics.Blueprint_PredictProjectilePath_Advanced` (make `PredictProjectilePathParams` (`SceneComponent.K2_GetComponentLocation` (`self.SpawnPoint`)) (* (`SceneComponent.GetForwardVector` (`self.SpawnPoint`)) 10000.0) true 0.0 5.0 false "ECC_WorldStatic" (`|MakeArray` "ObjectTypeQuery1" :!type "EObjectTypeQuery Enum") (`|MakeArray` self :!type "Actor Object Reference") 20.0 0.0 "ForOneFrame")))

(fn `UserConstructionScript`)