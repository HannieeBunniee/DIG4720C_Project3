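; Main game mode that builds lane waypoint routes and spawns AI minion waves at every spawn point.
; On BeginPlay it sorts waypoints into team/lane arrays by order, forward and reversed, served by GetWaypointsForMinion; Team0Lane1 is never filled, as lane 1 writes to Team1Lane0.
; Two looping timers share a DoN: one-second ticks spawn up to five minions per point, and the wave timer resets the count.
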(event `self.ReceiveBeginPlay`
  (bind _waypointcounts (`self.WaypointCounts`))
  (bind _waypointcounts_2 (`self.WaypointCounts`))
  (`|ExecutionSequence`
    (:`then_0`
      (bind _outactors (`GameplayStatics.GetAllActorsOfClass` "/Game/Blueprints/Enemy/Actors/BP_Waypoint.BP_Waypoint_C"))
      (`KismetArrayLibrary.Array_Clear` _waypointcounts_2)
      (`KismetArrayLibrary.Array_Resize` _waypointcounts_2 2)
      (for _array_element _outactors
        (bind _lane (`/Game/Blueprints/Enemy/Actors/BP_Waypoint.Lane` _array_element))
        (bind _result (`/Engine/EditorBlueprintResources/StandardMacros.IncrementInt` (`|GetArrayItem` _waypointcounts _lane))
          (:`  `
            (`KismetArrayLibrary.Array_Set` _waypointcounts _lane _result))))
      (for _array_element_2 _outactors
        (bind _lane_2 (`/Game/Blueprints/Enemy/Actors/BP_Waypoint.Lane` _array_element_2))
        (switch `int` _lane_2
          (:`0`
            (bind _waypointorder (`/Game/Blueprints/Enemy/Actors/BP_Waypoint.WaypointOrder` _array_element_2))
            (`KismetArrayLibrary.Array_Set` (`self.Team0Lane0`) _waypointorder)
            (bind _returnvalue (- (- (`|GetArrayItem` (`self.WaypointCounts`) _lane_2) 1) _waypointorder))
            (`KismetArrayLibrary.Array_Set` (`self.Team1Lane0`) _returnvalue))
          (:`1`
            (`KismetArrayLibrary.Array_Set` (`self.Team1Lane0`) _waypointorder)
            (`KismetArrayLibrary.Array_Set` (`self.Team1Lane1`) _returnvalue)))))
    (:`then_1`
      (bind _outactors_2 (`GameplayStatics.GetAllActorsOfClass` "/Game/Blueprints/Enemy/Actors/BP_MinionSpawnPoint.BP_MinionSpawnPoint_C"))
      (set `self.MinionSpawns` _outactors_2))
    (:`then_2`
      (`KismetSystemLibrary.Delay` 1.0)
      (`KismetSystemLibrary.K2_SetTimerDelegate` (delegate `SpawnSubWave`) 1.0 true)
      (`KismetSystemLibrary.K2_SetTimerDelegate` (delegate `SpawnMinionWave`) (`self.WaveSpawnTimer`) true))))

(event `SpawnMinionWave`
  (bind _minionspawns (`self.MinionSpawns`))
  (goto _label :!via `Reset`))

(event `SpawnSubWave`
  (bind _minionspawns (`self.MinionSpawns`))
  (`/Engine/EditorBlueprintResources/StandardMacros.Do N` 5 :!label _label
    (:`Exit`
      (for _index (range (+ (`KismetArrayLibrary.Array_LastIndex` _minionspawns) 1))
        (bind (_returnvalue_location _returnvalue_rotation) (`KismetMathLibrary.BreakTransform` (`self.GetTransform` (`|GetArrayItem` _minionspawns _index))))
        (bind _returnvalue (`AIBlueprintHelperLibrary.SpawnAIFromClass` "/Game/Blueprints/Enemy/Units/BP_Minion.BP_Minion_C" "/Game/Blueprints/Enemy/AI/BT_MinionAI.BT_MinionAI" _returnvalue_location _returnvalue_rotation false null))
        (bind _asbp_minion (cast `/Game/Blueprints/Enemy/Units/BP_Minion` _returnvalue))
        (`KismetArrayLibrary.Array_Add` (`self.MinionArray`) _asbp_minion)))))

(fn `GetWaypointsForMinion`
  (params (Team :type Integer) (Lane :type Integer))
  (returns (Waypoint :type "Array of /Game/Blueprints/Enemy/Actors/BP_Waypoint Object Reference"))
  (return (select `int` (+ (* Team 2) Lane) :`0` (`self.Team0Lane0`) :`1` (`self.Team1Lane0`) :`2` (`self.Team0Lane1`) :`3` (`self.Team1Lane1`))))

(fn `UserConstructionScript`)