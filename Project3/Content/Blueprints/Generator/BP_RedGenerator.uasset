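; BP_RedGenerator is a destructible generator actor that shields the red nexus until it is destroyed.
; Any damage it takes is subtracted from its current health.
; At zero health it prints an "enemy nexus is open" message, enables query and physics collision on the Box of the BP_RedNexus found in the level, then destroys itself.
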(event `self.ReceiveAnyDamage`
  (params (Damage :type "Float (single-precision)") (DamageType :type "DamageType Object Reference") (InstigatedBy :type "Controller Object Reference") (DamageCauser :type "Actor Object Reference"))
  (set `self.Current Health` (- (`self.Current Health`) Damage))
  (if (<= (`self.Current Health`) 0.0)
    (`KismetSystemLibrary.PrintString` "ENEMY NEXUS IS OPEN!")
    (bind _returnvalue (`GameplayStatics.GetActorOfClass` "/Game/Blueprints/Nexus/BP_RedNexus.BP_RedNexus_C"))
    (`PrimitiveComponent.SetCollisionEnabled` (`/Game/Blueprints/Nexus/BP_RedNexus.Box` _returnvalue) "QueryAndPhysics")
    (`self.K2_DestroyActor`)))

(fn `UserConstructionScript`)