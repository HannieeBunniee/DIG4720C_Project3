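; BP_BlueGenerator is a destructible generator that guards the blue Nexus until its health runs out.
; Any damage is subtracted from its current health.
; At zero or below, it prints a warning that the Nexus is open, finds BP_BlueNexus by class, and enables query and physics collision on its box.
; It also sets the Nexus health widget from its stored reference, then destroys itself.
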(event `self.ReceiveAnyDamage`
  (params (Damage :type "Float (single-precision)") (DamageType :type "DamageType Object Reference") (InstigatedBy :type "Controller Object Reference") (DamageCauser :type "Actor Object Reference"))
  (set `self.Current Health` (- (`self.Current Health`) Damage))
  (if (<= (`self.Current Health`) 0.0)
    (`KismetSystemLibrary.PrintString` "YOUR NEXUS IS OPEN!")
    (bind _returnvalue (`GameplayStatics.GetActorOfClass` "/Game/Blueprints/Nexus/BP_BlueNexus.BP_BlueNexus_C"))
    (`PrimitiveComponent.SetCollisionEnabled` (`/Game/Blueprints/Nexus/BP_BlueNexus.Box` _returnvalue) "QueryAndPhysics")
    (`WidgetComponent.SetWidget` (`/Game/Blueprints/Nexus/BP_BlueNexus.HealthWidget` _returnvalue) (`/Game/Blueprints/Nexus/BP_BlueNexus.widget ref` _returnvalue))
    (`self.K2_DestroyActor`)))

(fn `UserConstructionScript`)