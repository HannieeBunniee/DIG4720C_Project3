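; BP_MainMenu is an actor that glides back and forth between two fixed points, apparently as a moving main menu camera.
; From BeginPlay, the T_MoveCamera timeline lerps the actor's location along the Y axis.
; On finish, a FlipFlop toggles IsForward and re-enters the shared branch through Play or Reverse, replaying or reversing the timeline in an endless ping-pong.
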(event `self.ReceiveBeginPlay`
  (`self.Play`))

(event `Play`
  (if (`self.IsForward`) :!label _label
    (bind (_direction _alpha) (`Timeline|T_MoveCamera` :!via `PlayFromStart` :!label _label_2)
      (:`Update`
        (`self.K2_SetActorLocation` (`KismetMathLibrary.VLerp` (3040.0 -1035.0 1992.0) (3040.0 400.0 1992.0) _alpha)))
      (:`Finished`
        (`/Engine/EditorBlueprintResources/StandardMacros.FlipFlop`
          (:`A`
            (set `self.IsForward` false)
            (`self.Reverse`))
          (:`B`
            (set `self.IsForward` true)
            (`self.Play`)))))
    (else
      (goto _label_2 :!via `Reverse`))))

(event `Reverse`
  (goto _label))

(fn `UserConstructionScript`)