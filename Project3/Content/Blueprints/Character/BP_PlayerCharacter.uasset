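; Player tank character that drives, aims a separate turret and barrel, fires projectiles, and handles the HUD, pause menu and game over.
; Firing spawns a projectile with sound and camera shakes, gated by a recoil timeline and reload delay.
; Move or look input triggers a debug-drawn trajectory prediction using a hard-coded launch speed.
; Damage reduces health until defeat; meteor-rain spawning is defined, but its timer is disconnected.
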(event `InputAction|FirePrimary`
  (params (Key :type "Key Structure"))
  (bind _returnvalue (`self.K2_GetActorLocation`))
  ;[1 1 1] Shoot
  (:`Pressed`
    (if (`self.IsDoneShooting`)
      (`|SpawnActorFromClass` "/Game/Blueprints/Projectiles/BP_PlayerProjectile.BP_PlayerProjectile_C" (`KismetMathLibrary.MakeTransform` (`SceneComponent.K2_GetComponentLocation` (`self.SpawnPoint`)) (`SceneComponent.K2_GetComponentRotation` (`self.SpawnPoint`))) "Undefined" "OverrideRootScale" null null)
      ;[1 1 1] Camera Shake & Sound
      (`GameplayStatics.PlayWorldCameraShake` "/Game/Blueprints/BP_CameraShakeShoot.BP_CameraShakeShoot_C" _returnvalue 0.0 500.0)
      (`GameplayStatics.PlaySoundAtLocation` (`KismetArrayLibrary.Array_Random` (`self.Sound`)) _returnvalue (struct) 1.0 1.0 0.0 null null null)
      ;[1 1 1] Recoil Animation & Reload Shake
      (set `self.IsDoneShooting` false)
      (bind (_direction _alpha) (`Timeline|T_GunRecoil` :!via `PlayFromStart` :!label _label)
        (:`Update`
          (`SceneComponent.K2_SetRelativeLocation` (`self.TankGuns`) (`KismetMathLibrary.VLerp` (0.0 0.0 0.0) (0.0 -90.0 0.0) _alpha) false false))
        (:`Finished`
          (if (not (`self.IsDoneShooting`))
            (`self.Recoil`)
            (`KismetSystemLibrary.Delay` 1.0)
            (set `self.IsDoneShooting` true)
            (`GameplayStatics.PlayWorldCameraShake` "/Game/Blueprints/BP_CameraShakeReload.BP_CameraShakeReload_C" (`self.K2_GetActorLocation`) 0.0 500.0)))))))

(event `Recoil`
  ;[1 1 1] Recoil Animation & Reload Shake
  (goto _label :!via `ReverseFromEnd`))

(event `self.ReceiveTick`
  (params (DeltaSeconds :type "Float (single-precision)"))
  ;[1 1 1] Have dots when player move/looks
  (if (or (!= (`self.GetInputAxisValue`) 0.0) (!= (`self.GetInputAxisValue`) 0.0) (!= (`self.GetInputAxisValue`) 0.0) (!= (`self.GetInputAxisValue`) 0.0))
    (`self.Aiming Dots`)))

(event `self.ReceiveAnyDamage`
  (params (Damage :type "Float (single-precision)") (DamageType :type "DamageType Object Reference") (InstigatedBy :type "Controller Object Reference") (DamageCauser :type "Actor Object Reference"))
  ;[1 1 1] Taking Damage
  (set `self.CurrentHealth` (- (`self.CurrentHealth`) Damage))
  (if (<= (`self.CurrentHealth`) 0.0)
    ;;[1 1 1] Lose Screen
    (bind _returnvalue (`|CreateWidget` "/Game/Widget/UI_GameOver.UI_GameOver_C"))
    (`UserWidget.AddToViewport` _returnvalue 0)
    (set `PlayerController.bShowMouseCursor` true (`GameplayStatics.GetPlayerController` 0))
    (`GameplayStatics.SetGamePaused` true)
    (`GameplayStatics.PlaySound2D` "/Game/Sounds/SFX/Defeat2.Defeat2" 1.0 1.0 0.0 null null)))

(event `InputAxis|MoveForward`
  (params (AxisValue :type "Float (single-precision)"))
  ;[1 1 1] Movement
  (`self.AddMovementInput` (`KismetMathLibrary.GetForwardVector` (`KismetMathLibrary.MakeRotator` (.roll (`Controller.GetControlRotation` (`self.GetController`))) (.pitch (`Controller.GetControlRotation` (`self.GetController`))) (+ (.yaw (`Controller.GetControlRotation` (`self.GetController`))) (* (stale `InputAxis|MoveRight` AxisValue) (`self.TurnSpeed`))))) AxisValue))

(event `self.ReceiveBeginPlay`
  (`|ExecutionSequence`
    (:`then_0`
      ;[1 1 1] Player HP
      (if (not (`self.IsMainMenu?`))
        (bind _returnvalue (`|CreateWidget` "/Game/Widget/UI_PlayerHUD.UI_PlayerHUD_C"))
        (`UserWidget.AddToViewport` _returnvalue 0)))
    (:`then_1`)))

(event `InputAxis|MoveRight`
  (params (AxisValue :type "Float (single-precision)"))
  (bind _returnvalue (`self.GetController`))
  ;[1 1 1] Movement
  (`Controller.SetControlRotation` _returnvalue (`KismetMathLibrary.MakeRotator` (.roll (`Controller.GetControlRotation` _returnvalue)) (.pitch (`Controller.GetControlRotation` _returnvalue)) (+ (.yaw (`Controller.GetControlRotation` _returnvalue)) (* AxisValue (`self.TurnSpeed`))))))

(event `InputAxis|LookRight`
  (params (AxisValue :type "Float (single-precision)"))
  ;[1 1 1] Looking
  (`SceneComponent.K2_AddLocalRotation` (`self.TankTurret`) (`KismetMathLibrary.MakeRotator` 0.0 0.0 (* AxisValue (`self.LookSpeedX`))) false false))

(event `InputAxis|LookUp`
  (params (AxisValue :type "Float (single-precision)"))
  ;[1 1 1] Looking
  (`SceneComponent.K2_AddLocalRotation` (`self.TankBarrel`) (`KismetMathLibrary.MakeRotator` (* AxisValue (`self.LookSpeedY`))) false false))

(event `InputAction|Pause`
  (params (Key :type "Key Structure"))
  (bind _returnvalue (`GameplayStatics.GetPlayerController` 0))
  ;[1 1 1] Pause
  (:`Pressed`
    (`/Engine/EditorBlueprintResources/StandardMacros.IsValid` (`self.PauseMenu`)
      (:`Is Valid`
        _)
      (:`Is Not Valid`
        (bind _returnvalue_2 (`|CreateWidget` "/Game/Widget/UI_PauseMenu.UI_PauseMenu_C"))
        (bind _output_get (set `self.PauseMenu` _returnvalue_2))))
    (set `PlayerController.bShowMouseCursor` true _returnvalue)
    (`WidgetBlueprintLibrary.SetInputMode_GameAndUIEx` _returnvalue _output_get)
    (`UserWidget.AddToViewport` _output_get 0)
    (`GameplayStatics.SetGamePaused` true)))

(fn `Aiming Dots`
  (`GameplayStatics.Blueprint_PredictProjectilePath_Advanced` (make `PredictProjectilePathParams` (`SceneComponent.K2_GetComponentLocation` (`self.SpawnPoint`)) (* (`SceneComponent.GetForwardVector` (`self.SpawnPoint`)) 10000.0) true 0.0 5.0 false "ECC_WorldStatic" (`|MakeArray` "ObjectTypeQuery1" :!type "EObjectTypeQuery Enum") (`|MakeArray` self :!type "Actor Object Reference") 20.0 0.0 "ForOneFrame")))

(fn `GetRandomLocationInRadius`
  (params (Origin :type "Vector Structure") (Radius :type "Float (double-precision)"))
  (returns (ReturnValue :type "Vector Structure"))
  ;[1 1 1] DO NOT CHANGE THIS!
  (return (+ Origin (* (`KismetMathLibrary.GreaterGreater_VectorRotator` (0.0 0.0 0.0) (`KismetMathLibrary.MakeRotator` 0.0 0.0 (`KismetMathLibrary.RandomFloatInRange` 0.0 360.0))) (`KismetMathLibrary.RandomFloatInRange` 0.0 Radius)))))

(fn `SpawnMeteor`
  (bind _returnvalue (`self.GetRandomLocationInRadius` (+ (`SceneComponent.K2_GetComponentLocation` (`self.MeteorSpawnPoint`)) (0.0 0.0 1000.0)) 500.0))
  (`KismetSystemLibrary.DrawDebugSphere` _returnvalue 20.0 12 (struct :`R` 1.0 :`G` 1.0 :`B` 1.0 :`A` 1.0) 1.0 1.0)
  (`|SpawnActorFromClass` "/Game/Blueprints/Projectiles/BP_BulletRainProjectile.BP_BulletRainProjectile_C" (`KismetMathLibrary.MakeTransform` _returnvalue (struct :`Pitch` -90.0)) "Undefined" "OverrideRootScale" null null))

(fn `UserConstructionScript`)