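; BP_PlayerProjectile is the player's explosive projectile, which deals area damage when it touches another actor.
; A capsule overlap with anything other than the player character applies full, no-falloff radial damage around the projectile, ignoring the player.
; It then spawns a blue Niagara explosion at the bullet component's location and destroys itself.
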(event `self.Capsule.OnComponentBeginOverlap`
  (params (OverlappedComponent :type "PrimitiveComponent Object Reference") (OtherActor :type "Actor Object Reference") (OtherComp :type "PrimitiveComponent Object Reference") (OtherBodyIndex :type Integer) (bFromSweep :type Boolean) (SweepResult :type "HitResult Structure (by ref)"))
  (bind _returnvalue (`GameplayStatics.GetPlayerCharacter` 0))
  (if (!= OtherActor _returnvalue)
    (`GameplayStatics.ApplyRadialDamage` (`self.Damage`) (`self.K2_GetActorLocation` self) 500.0 null (`|MakeArray` _returnvalue :!type "Actor Object Reference") null null true)
    (`NiagaraFunctionLibrary.SpawnSystemAtLocation` "/Game/Particles/PS_Explosion_SystemBLUE.PS_Explosion_SystemBLUE" (`SceneComponent.K2_GetComponentLocation` (`self.Bullet`)))
    (`self.K2_DestroyActor`)))

(fn `UserConstructionScript`)