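; Proximity turret enemy that activates while the player is inside its AttackRange, loses health from damage and destroys itself at zero.
; Activation plays a sound, switches eye material and light color, and starts CombatTimeline; leaving range reverses the color and stops it.
; Timeline updates smoothly turn the head toward the player, while a Delay throttles BP_EnemyProjectile spawns tinted to the active eye color.
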(event `self.ReceiveAnyDamage`
  (params (Damage :type "Float (single-precision)") (DamageType :type "DamageType Object Reference") (InstigatedBy :type "Controller Object Reference") (DamageCauser :type "Actor Object Reference"))
  ;[1 1 1] Take Damage
  (bind _output_get (set `self.CurrentHealth` (- (`self.CurrentHealth`) Damage)))
  (if (<= _output_get 0.0)
    (`self.K2_DestroyActor`)))

(event `Activate`
  ;[1 1 1] Activate/Deactivate shooting
  (`self.UpdateEyeColor` (`self.Activated Eye Color`))
  (set `self.Activated?` true)
  (`GameplayStatics.SpawnSoundAtLocation` null (`self.K2_GetActorLocation`) (struct) 1.0 1.0 0.0 null null) ; play sound when player come near
  (`Timeline|Combat Timeline` :!label _label
    (:`Update`
      (`|ExecutionSequence`
        (:`then_0`
          (`self.LookAtPlayer`))
        (:`then_1`
          (`KismetSystemLibrary.Delay` (`self.FireRate`))
          (if (`self.Activated?`)
            (`self.SpawnProjectileAtPlayer`)))))))

(event `Deactivate`
  ;[1 1 1] Activate/Deactivate shooting
  (`self.UpdateEyeColor` (`self.Deactivated Eye Color`))
  (set `self.Activated?` false)
  (goto _label :!via `Stop`))

(event `self.AttackRange.OnComponentBeginOverlap`
  (params (OverlappedComponent :type "PrimitiveComponent Object Reference") (OtherActor :type "Actor Object Reference") (OtherComp :type "PrimitiveComponent Object Reference") (OtherBodyIndex :type Integer) (bFromSweep :type Boolean) (SweepResult :type "HitResult Structure (by ref)"))
  ;[1 1 1] Event overlapse and exit
  (if (== OtherActor (`GameplayStatics.GetPlayerCharacter` 0))
    (`self.Activate`)))

(event `self.AttackRange.OnComponentEndOverlap`
  (params (OverlappedComponent :type "PrimitiveComponent Object Reference") (OtherActor :type "Actor Object Reference") (OtherComp :type "PrimitiveComponent Object Reference") (OtherBodyIndex :type Integer))
  ;[1 1 1] Event overlapse and exit
  (if (== OtherActor (`GameplayStatics.GetPlayerCharacter` 0))
    (`self.Deactivate`)))

(fn `LookAtPlayer`
  (`SceneComponent.K2_SetWorldRotation` (`self.Head`) (`KismetMathLibrary.RLerp` (`SceneComponent.K2_GetComponentRotation` (`self.Head`)) (`KismetMathLibrary.FindLookAtRotation` (`SceneComponent.K2_GetComponentLocation` (`self.Head`)) (`self.K2_GetActorLocation` (`GameplayStatics.GetPlayerPawn` 0))) 0.5) false false))

(fn `SpawnProjectileAtPlayer`
  ;[1 1 1] Spawn bullets
  (bind _returnvalue (`|SpawnActorFromClass` "/Game/Blueprints/Projectors/BP_EnemyProjectile.BP_EnemyProjectile_C" (`SceneComponent.K2_GetComponentToWorld` (`self.SpawnPoint`)) "Undefined" "OverrideRootScale" null null))
  ;[1 1 1] Set Bullet color
  (bind _returnvalue_2 (`PrimitiveComponent.CreateDynamicMaterialInstance` (`/Game/Blueprints/Projectors/BP_EnemyProjectile.Bullet` _returnvalue) 0 "/Game/Blueprints/ProximityTurret/M_ProximityTurretEye.M_ProximityTurretEye" "None"))
  (`MaterialInstanceDynamic.SetVectorParameterValue` _returnvalue_2 "Colour" (`self.Activated Eye Color`)))

(fn `UpdateEyeColor`
  (params (Colour :type "LinearColor Structure"))
  (`MaterialInstanceDynamic.SetVectorParameterValue` (`self.DynamicEyeMaterial`) "Colour" Colour)
  (`LightComponent.SetLightColor` (`self.Light`) Colour true))

(fn `UserConstructionScript`
  ;[1 1 1] Eye Material
  (bind _returnvalue (`PrimitiveComponent.CreateDynamicMaterialInstance` (`self.Eye`) 0 "/Game/Blueprints/ProximityTurret/M_ProximityTurretEye.M_ProximityTurretEye" "None"))
  (bind _output_get (set `self.DynamicEyeMaterial` _returnvalue))
  (`MaterialInstanceDynamic.SetVectorParameterValue` _output_get "Colour" (`self.Deactivated Eye Color`))
  ;[1 1 1] Eye Color
  (`LightComponent.SetLightColor` (`self.Light`) (`self.Deactivated Eye Color`) true))