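; BP_TurretTest is a proximity turret test Blueprint that reacts to player characters entering its AttackRange.
; Overlap events maintain ActorsInRange, calling Activate on each entry and Deactivate when no valid first entry remains.
; Activate snaps the Head toward the first tracked player once per call, without continuous tracking.
; The construction script tints a dynamic eye material and light with the deactivated colour; Fire and Deactivate only print debug text.
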(event `Activate`
  (bind _output (`|GetArrayItem` (`self.Actors in Range`)))
  (`KismetSystemLibrary.PrintString` "activated")
  (`/Engine/EditorBlueprintResources/StandardMacros.IsValid` _output
    (:`Is Valid`
      (`SceneComponent.K2_SetWorldRotation` (`self.Head`) (`KismetMathLibrary.FindLookAtRotation` (`self.K2_GetActorLocation`) (`self.K2_GetActorLocation` _output)) false false))))

(event `Deactivate`
  (`KismetSystemLibrary.PrintString` "deactivated"))

(event `self.AttackRange.OnComponentBeginOverlap`
  (params (OverlappedComponent :type "PrimitiveComponent Object Reference") (OtherActor :type "Actor Object Reference") (OtherComp :type "PrimitiveComponent Object Reference") (OtherBodyIndex :type Integer) (bFromSweep :type Boolean) (SweepResult :type "HitResult Structure (by ref)"))
  (bind _asbp_player_character (cast `/Game/Blueprints/Character/BP_PlayerCharacter` OtherActor))
  (`KismetArrayLibrary.Array_Add` (`self.Actors in Range`) _asbp_player_character)
  (`self.Activate`))

(event `self.AttackRange.OnComponentEndOverlap`
  (params (OverlappedComponent :type "PrimitiveComponent Object Reference") (OtherActor :type "Actor Object Reference") (OtherComp :type "PrimitiveComponent Object Reference") (OtherBodyIndex :type Integer))
  (bind _actors_in_range (`self.Actors in Range`))
  (bind _asbp_player_character (cast `/Game/Blueprints/Character/BP_PlayerCharacter` OtherActor))
  (`KismetArrayLibrary.Array_RemoveItem` _actors_in_range _asbp_player_character)
  (`/Engine/EditorBlueprintResources/StandardMacros.IsValid` (`|GetArrayItem` _actors_in_range)
    (:`Is Not Valid`
      (`self.Deactivate`))))

(fn `Fire`
  (`KismetSystemLibrary.PrintString` "i tried to fire"))

(fn `UserConstructionScript`
  ;[1 1 1] Eye Material
  (bind _returnvalue (`PrimitiveComponent.CreateDynamicMaterialInstance` (`self.Eye`) 0 "/Game/Blueprints/ProximityTurret/M_ProximityTurretEye.M_ProximityTurretEye" "None"))
  (bind _output_get (set `self.DynamicEyeMaterial` _returnvalue))
  (`MaterialInstanceDynamic.SetVectorParameterValue` _output_get "Colour" (`self.Deactivated Eye Color`))
  ;[1 1 1] Eye Color
  (`LightComponent.SetLightColor` (`self.Light`) (`self.Deactivated Eye Color`) true))