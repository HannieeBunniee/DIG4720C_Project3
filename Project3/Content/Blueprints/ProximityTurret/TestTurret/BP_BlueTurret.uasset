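; Blue turret actor that targets minions and players carrying the AttackTeam tag inside its AttackRange.
; Overlaps maintain ActorsInRange; a Timeline aims TurretGun at the first entry and fires twin projectiles through a FireRate Delay.
; An empty range stops the Timeline, though Deactivate still leaves Activated true.
; Damage updates a health widget, shown when players enter range, and destroys the turret at zero.
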(event `self.ReceiveBeginPlay`
  (`|ExecutionSequence`
    (:`then_0`
      (bind _returnvalue (`|CreateWidget` "/Game/Widget/UI_TurretHeath.UI_TurretHeath_C"))
      (set `self.Widget Ref` _returnvalue))
    (:`then_1`
      (`KismetArrayLibrary.Array_Clear` (`self.Actors In Range`)))))

(event `self.ReceiveAnyDamage`
  (params (Damage :type "Float (single-precision)") (DamageType :type "DamageType Object Reference") (InstigatedBy :type "Controller Object Reference") (DamageCauser :type "Actor Object Reference"))
  (bind _output_get (set `self.CurrentHealth` (- (`self.CurrentHealth`) Damage)))
  (`/Game/Widget/UI_TurretHeath.update HP bar` (`self.Widget Ref`) (`self.CurrentHealth`) (`self.MaxHealth`))
  (if (<= _output_get 0.0)
    (`self.K2_DestroyActor`)
    (else
      (`KismetSystemLibrary.PrintString` "Turret Damaged"))))

(event `Activate`
  (set `self.Activated` true)
  (`Timeline|Timeline_0` :!label _label
    (:`Update`
      (`|ExecutionSequence`
        (:`then_0`
          (`self.LookAtPlayer`))
        (:`then_1`
          (`KismetSystemLibrary.Delay` (`self.FireRate`))
          (if (`self.Activated`)
            (`self.ShootAtPlayer`)))))))

(event `Deactivate`
  (set `self.Activated` true)
  (goto _label :!via `Stop`))

(event `self.AttackRange.OnComponentBeginOverlap`
  (params (OverlappedComponent :type "PrimitiveComponent Object Reference") (OtherActor :type "Actor Object Reference") (OtherComp :type "PrimitiveComponent Object Reference") (OtherBodyIndex :type Integer) (bFromSweep :type Boolean) (SweepResult :type "HitResult Structure (by ref)"))
  (bind _asbp_minion (cast `/Game/Blueprints/Enemy/Units/BP_Minion` OtherActor)
    (:`then`
      (if (`self.ActorHasTag` _asbp_minion (`self.AttackTeam`))
        (`KismetArrayLibrary.Array_Add` (`self.Actors In Range`) _asbp_minion)
        (`self.Activate`)))
    (:`CastFailed`
      (bind _asbp_player_character (cast `/Game/Blueprints/Character/BP_PlayerCharacter` OtherActor))
      (`UserWidget.AddToViewport` (`self.Widget Ref`) 0)
      (if (`self.ActorHasTag` _asbp_player_character (`self.AttackTeam`))
        (`KismetArrayLibrary.Array_Add` (`self.Actors In Range`) _asbp_player_character)
        (`self.Activate`)))))

(event `self.AttackRange.OnComponentEndOverlap`
  (params (OverlappedComponent :type "PrimitiveComponent Object Reference") (OtherActor :type "Actor Object Reference") (OtherComp :type "PrimitiveComponent Object Reference") (OtherBodyIndex :type Integer))
  (bind _actors_in_range (`self.Actors In Range`))
  (cast `/Game/Blueprints/Character/BP_PlayerCharacter` OtherActor
    (:`then`
      (bind _foundwidgets (`WidgetBlueprintLibrary.GetAllWidgetsOfClass` "/Game/Widget/UI_TurretHeath.UI_TurretHeath_C"))
      (`Widget.RemoveFromParent` _foundwidgets))
    (:`CastFailed`
      _))
  (if (`self.ActorHasTag` OtherActor (`self.AttackTeam`))
    (`KismetArrayLibrary.Array_RemoveItem` _actors_in_range OtherActor)
    (`/Engine/EditorBlueprintResources/StandardMacros.IsValid` (`|GetArrayItem` _actors_in_range)
      (:`Is Not Valid`
        (`self.Deactivate`)))))

(fn `LookAtPlayer`
  (bind _output (`|GetArrayItem` (`self.Actors In Range`)))
  (`/Engine/EditorBlueprintResources/StandardMacros.IsValid` _output
    (:`Is Valid`
      (`SceneComponent.K2_SetWorldRotation` (`self.TurretGun`) (`KismetMathLibrary.FindLookAtRotation` (`SceneComponent.K2_GetComponentLocation` (`self.TurretGun`)) (`self.K2_GetActorLocation` _output)) false false))))

(fn `ShootAtPlayer`
  (bind (_returnvalue_location _returnvalue_rotation _returnvalue_scale) (`KismetMathLibrary.BreakTransform` (`SceneComponent.K2_GetComponentToWorld` (`self.SpawnPointLeft`))))
  (bind (_returnvalue_location_2 _returnvalue_rotation_2 _returnvalue_scale_2) (`KismetMathLibrary.BreakTransform` (`SceneComponent.K2_GetComponentToWorld` (`self.SpawnPointRight`))))
  (`|SpawnActorFromClass` "/Game/Blueprints/Projectiles/BP_TurretProjectileBLUE.BP_TurretProjectileBLUE_C" (`KismetMathLibrary.MakeTransform` _returnvalue_location_2 _returnvalue_rotation_2 _returnvalue_scale_2) "AlwaysSpawn" "OverrideRootScale" null null)
  (`|SpawnActorFromClass` "/Game/Blueprints/Projectiles/BP_TurretProjectileBLUE.BP_TurretProjectileBLUE_C" (`KismetMathLibrary.MakeTransform` _returnvalue_location _returnvalue_rotation _returnvalue_scale) "AlwaysSpawn" "OverrideRootScale" null null))

(fn `UserConstructionScript`)