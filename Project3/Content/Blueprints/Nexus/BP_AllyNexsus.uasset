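; BP_AllyNexsus is the allied nexus, whose destruction loses the game.
; Its AnyDamage event subtracts incoming damage from CurrentHealth.
; When health reaches zero or below, it adds the UI_GameOver widget to the viewport, shows the first player's mouse cursor and pauses the game.
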(event `self.ReceiveAnyDamage`
  (params (Damage :type "Float (single-precision)") (DamageType :type "DamageType Object Reference") (InstigatedBy :type "Controller Object Reference") (DamageCauser :type "Actor Object Reference"))
  (set `self.CurrentHealth` (- (`self.CurrentHealth`) Damage))
  (if (<= (`self.CurrentHealth`) 0.0)
    ;[1 1 1] Lose
    (bind _returnvalue (`|CreateWidget` "/Game/Widget/UI_GameOver.UI_GameOver_C"))
    (`UserWidget.AddToViewport` _returnvalue 0)
    (set `PlayerController.bShowMouseCursor` true (`GameplayStatics.GetPlayerController` 0))
    (`GameplayStatics.SetGamePaused` true)))

(fn `UserConstructionScript`)